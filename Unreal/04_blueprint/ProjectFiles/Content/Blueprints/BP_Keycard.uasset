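; BP_Keycard is a collectible keycard that changes colour when the player character is nearby and can be picked up.
; Box overlap with BP_Character swaps the KeyCard material to M_FlatBase until collection, and ending overlap restores M_FlatKey.
; Interact snaps the keycard to the supplied target point, keeping relative scale, then marks it collected, restores M_FlatKey and returns false.
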(event OnComponentBeginOverlap(Box)
  (params (OverlappedComponent :type Primitive%20Component%20Object%20Reference) (OtherActor :type Actor%20Object%20Reference) (OtherComp :type Primitive%20Component%20Object%20Reference) (OtherBodyIndex :type Integer) (bFromSweep :type Boolean) (SweepResult :type Hit%20Result%20Structure%20%28by%20ref%29))
  ;[1 1 1] Overlap Events to Change Colour (Before Collection)
  (if (not (Variables|Default|GetbBeenCollected))
    (Utilities|Casting|CastToBP_Character OtherActor)
    (Rendering|Material|SetMaterial (Variables|Default|GetKeyCard) 0 "/Game/Assets/Material/M_FlatBase.M_FlatBase")))

(event OnComponentEndOverlap(Box)
  (params (OverlappedComponent :type Primitive%20Component%20Object%20Reference) (OtherActor :type Actor%20Object%20Reference) (OtherComp :type Primitive%20Component%20Object%20Reference) (OtherBodyIndex :type Integer))
  ;[1 1 1] Overlap Events to Change Colour (Before Collection)
  (Utilities|Casting|CastToBP_Character OtherActor)
  (Rendering|Material|SetMaterial (Variables|Default|GetKeyCard) 0 "/Game/Assets/Material/M_FlatKey.M_FlatKey"))

(fn ConstructionScript)

(fn Interact
  (params (TargetPoint :type Scene%20Component%20Object%20Reference))
  (Transformation|AttachComponentToComponent TargetPoint "None" "SnapToTarget" "SnapToTarget" "KeepRelative" true)
  (Variables|Default|SetbBeenCollected true)
  (Rendering|Material|SetMaterial (Variables|Default|GetKeyCard) 0 "/Game/Assets/Material/M_FlatKey.M_FlatKey")
  (return false))