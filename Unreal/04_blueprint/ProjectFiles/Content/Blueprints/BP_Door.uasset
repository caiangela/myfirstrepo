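; BP_Door is an interactable door that a BP_Keycard unlocks.
; Its box overlap swaps a material slot while a BP_Character is in range, and stores any overlapping keycard while setting CanUnlock, which is never cleared here.
; When unlockable, Interact passes KeycardSlot to the keycard's Interact, sets the material and calls OpenDoor.
; OpenDoor waits briefly, destroys the keycard, then rotates the mesh with a timeline.
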(event OnComponentBeginOverlap(Box)
  (params (OverlappedComponent :type Primitive%20Component%20Object%20Reference) (OtherActor :type Actor%20Object%20Reference) (OtherComp :type Primitive%20Component%20Object%20Reference) (OtherBodyIndex :type Integer) (bFromSweep :type Boolean) (SweepResult :type Hit%20Result%20Structure%20%28by%20ref%29))
  ;[1 1 1] Overlapping Event to Change Colour
  (Utilities|Casting|CastToBP_Character OtherActor
    (:then
      (Rendering|Material|SetMaterial (Variables|Debug|GetStaticMeshComponent) 1 "/Game/Assets/Material/M_FlatBase.M_FlatBase"))
    (:CastFailed
      (bind _asbp_keycard (Utilities|Casting|CastToBP_Keycard OtherActor))
      (Variables|Default|SetBP_KeyCard _asbp_keycard)
      (Variables|Default|SetbCanUnlock true))))

(event OnComponentEndOverlap(Box)
  (params (OverlappedComponent :type Primitive%20Component%20Object%20Reference) (OtherActor :type Actor%20Object%20Reference) (OtherComp :type Primitive%20Component%20Object%20Reference) (OtherBodyIndex :type Integer))
  ;[1 1 1] Overlapping Event to Change Colour
  (Utilities|Casting|CastToBP_Character OtherActor)
  (Rendering|Material|SetMaterial (Variables|Debug|GetStaticMeshComponent) 1 "/Game/Assets/Material/M_FlatPictureFrame.M_FlatPictureFrame"))

(event Custom|OpenDoor
  (Utilities|FlowControl|Delay 1.0)
  (Actor|DestroyActor (Variables|Default|GetBP_KeyCard))
  (bind _rotation (Timeline|Timeline_0 Play)
    (:Update
      (Transformation|SetWorldRotation (Variables|Debug|GetStaticMeshComponent) (Math|Rotator|MakeRotator 0.0 0.0 _rotation) false false))))

(event EventBeginPlay)

(event Collision|EventActorBeginOverlap
  (params (OtherActor :type Actor%20Object%20Reference)))

(event EventTick
  (params (DeltaSeconds :type Float%20%28single-precision%29)))

(fn ConstructionScript)

(fn Interact
  (params (TargetPoint :type Scene%20Component%20Object%20Reference))
  (if (Variables|Default|GetbCanUnlock)
    (Default|Interact (Variables|Default|GetBP_KeyCard) (Variables|Default|GetKeycardSlot))
    (Rendering|Material|SetMaterial (Variables|Debug|GetStaticMeshComponent) 1 "/Game/Assets/Material/M_FlatPictureFrame.M_FlatPictureFrame")
    (CallFunction|OpenDoor)
    (return false)))